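; MyCharacter is a character Blueprint that can pick up items into an inventory.
; Its Pickup event adds the item to MyInventory, then shows the item count and total weight in kilograms on a ThoughtBubble text.
; BeginPlay, overlap and Tick are unused disabled stubs, and the construction script only calls its parent.
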(event `Pickup`
  (params (Item :type "MyItem Object Reference"))
  (bind _myinventory (`self.MyInventory`))
  (`MyInventory.AddItem` _myinventory Item)
  (bind _returnvalue (`MyInventory.GetCount` _myinventory))
  (bind _returnvalue_2 (`MyInventory.GetWeights` _myinventory))
  (`ThoughtBubble.SetText` (`self.ThoughtBubble`) (`|FormatText` "{C} Items {W} kG" _returnvalue _returnvalue_2)))

(fn `UserConstructionScript`
  (`parent.UserConstructionScript`))